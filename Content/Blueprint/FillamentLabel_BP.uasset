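; Actor that displays a filament percentage as in-world text.
; Plus5% and Minus5% events step the Fillament value up or down by five, guarded to stay between zero and one hundred.
; Each change rewrites the TextRender component with the new value and a percent sign; nothing sets the text at start.
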(event Custom|Minus%205%25
  (if (> (Variables|Default|Getfillament) 0)
    (bind _output_get (Variables|Default|Setfillament (- (Variables|Default|Getfillament) 5)))
    (Rendering|Components|TextRender|SetText (Variables|Default|GetTextRender) (Utilities|Text|ToText(String) (Utilities|String|Append (Utilities|String|ToString(Integer) _output_get) "%")))))

(event Custom|Plus%205%25
  (if (< (Variables|Default|Getfillament) 100)
    (bind _output_get (Variables|Default|Setfillament (+ (Variables|Default|Getfillament) 5)))
    (Rendering|Components|TextRender|SetText (Variables|Default|GetTextRender) (Utilities|Text|ToText(String) (Utilities|String|Append (Utilities|String|ToString(Integer) _output_get) "%")))))

(event EventBeginPlay)

(event Collision|EventActorBeginOverlap
  (params (OtherActor :type Actor%20Object%20Reference)))

(event EventTick
  (params (DeltaSeconds :type Float%20%28single-precision%29)))

(fn ConstructionScript)