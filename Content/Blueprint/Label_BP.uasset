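; Label_BP is a text label that steps through entries in a Names array and shows the selected one on its TextRender.
; The Plus1 and Minus1 events move Index one step within a hard-coded 0 to 9 range, then set the text to the matching name.
; BeginPlay, Tick and the construction script are empty, so the Blueprint changes the text only through those two events.
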(event Custom|Minus%201
  (if (> (Variables|Default|Getindex) 0)
    (bind _output_get (Variables|Default|Setindex (- (Variables|Default|Getindex) 1)))
    (Rendering|Components|TextRender|SetText (Variables|Default|GetTextRender) (Utilities|Array|Get(acopy) (Variables|Default|GetNames) _output_get))))

(event Custom|Plus%201
  (if (< (Variables|Default|Getindex) 9)
    (bind _output_get (Variables|Default|Setindex (+ (Variables|Default|Getindex) 1)))
    (Rendering|Components|TextRender|SetText (Variables|Default|GetTextRender) (Utilities|Array|Get(acopy) (Variables|Default|GetNames) _output_get))))

(event EventBeginPlay)

(event Collision|EventActorBeginOverlap
  (params (OtherActor :type Actor%20Object%20Reference)))

(event EventTick
  (params (DeltaSeconds :type Float%20%28single-precision%29)))

(fn ConstructionScript)