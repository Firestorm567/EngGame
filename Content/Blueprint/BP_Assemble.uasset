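; BP_Assemble completes a drone construction task, swapping the assembled parts for a finished BP_Drone.
; When Assemble is called with exactly 23 BP_Grab actors overlapping, it destroys them and spawns the drone at a hardcoded location.
; It then blends the view to TPCCamera, hides the cursor, updates ThirdPersonCharacter's construction flags and calls RaiseMistake after a delay.
; Otherwise it prints the overlap count; Cube overlaps also print debug text.
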(event OnComponentBeginOverlap(Cube)
  (params (OverlappedComponent :type Primitive%20Component%20Object%20Reference) (OtherActor :type Actor%20Object%20Reference) (OtherComp :type Primitive%20Component%20Object%20Reference) (OtherBodyIndex :type Integer) (bFromSweep :type Boolean) (SweepResult :type Hit%20Result%20Structure%20%28by%20ref%29))
  (Development|PrintString (Utilities|GetDisplayName OverlappedComponent)))

(event Custom|Assemble
  (bind _returnvalue (Game|GetPlayerController 0))
  (bind _overlappingactors (Collision|GetOverlappingActors "/Game/Blueprint/BP_Grab.BP_Grab_C" :!class /Script/Engine.Actor))
  (bind _returnvalue_2 (Utilities|Array|Length _overlappingactors))
  (if (== _returnvalue_2 23)
    (Actor|DestroyActor _overlappingactors)
    (Game|SpawnActorfromClass "/Game/Blueprint/BP_Drone.BP_Drone_C" (Math|Transform|MakeTransform "-281.272675,324.879333,218.540802" "0, 0, 0" "1,1,1") "Undefined" 0 0)
    (Game|Player|SetViewTargetwithBlend _returnvalue (Variables|Default|GetTPC%20Camera) 1.0 "VTBlend_Linear" 0.0 false)
    (Variables|/Script/Engine.PlayerController|SetbShowMouseCursor _returnvalue false)
    (bind _asthird_person_character (Utilities|Casting|CastToThirdPersonCharacter (Game|Player|GetPlayerPawn 0)))
    (Variables|/Game/ThirdPersonBP/Blueprints/ThirdPersonCharacter.ThirdPersonCharacter_C|Setduringconstruction _asthird_person_character false)
    (Variables|/Game/ThirdPersonBP/Blueprints/ThirdPersonCharacter.ThirdPersonCharacter_C|Setall%20done _asthird_person_character true)
    (Utilities|FlowControl|Delay 3.0)
    (Default|RaiseMistake _asthird_person_character 7)
    (else
      (Development|PrintString (Utilities|String|ToString(Integer) _returnvalue_2)))))

(event EventBeginPlay)

(event Collision|EventActorBeginOverlap
  (params (OtherActor :type Actor%20Object%20Reference)))

(event EventTick
  (params (DeltaSeconds :type Float%20%28single-precision%29)))

(fn ConstructionScript)