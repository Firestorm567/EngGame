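; Printer button actor that spawns a selectable PickupObject_BP at a fixed world location.
; IndexChange steps CurrentIndex up or down, clamped to a hardcoded range of nine entries.
; Spawn passes itself to the new pickup, applies the mesh and index for that selection, then sets Blocked.
; While Blocked, Spawn only prints a debug string; nothing here clears the flag, and Press is empty.
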(event Custom|Spawn
  (bind _current_index (Variables|Default|Getcurrent_index))
  (if (Variables|Default|Getblocked)
    (Development|PrintString "2")
    (else
      (bind _returnvalue (Game|SpawnActorfromClass "/Game/Blueprint/PickupObject_BP.PickupObject_BP_C" (Math|Transform|MakeTransform "-240.000000,600.000000,241.750000") "Undefined" 0 0))
      (Default|Assign _returnvalue self)
      (Components|StaticMesh|SetStaticMesh (Variables|/Game/Blueprint/PickupObject_BP.PickupObject_BP_C|GetStaticMesh _returnvalue) (Utilities|Array|Get(acopy) (Variables|/Game/Blueprint/PickupObject_BP.PickupObject_BP_C|Getmesh_list _returnvalue) _current_index))
      (Variables|/Game/Blueprint/PickupObject_BP.PickupObject_BP_C|Setindex _returnvalue _current_index)
      (Variables|Default|Setblocked true))))

(event Custom|Press)

(event Custom|IndexChange
  (params (ispositive :type Boolean))
  (if ispositive
    (Variables|Default|Setcurrent_index (+ (Variables|Default|Getcurrent_index) 1))
    (if (== (Variables|Default|Getcurrent_index) 9)
      (Variables|Default|Setcurrent_index 8))
    (else
      (Variables|Default|Setcurrent_index (- (Variables|Default|Getcurrent_index) 1))
      (if (== (Variables|Default|Getcurrent_index) -1)
        (Variables|Default|Setcurrent_index 0)))))

(event EventBeginPlay)

(event Collision|EventActorBeginOverlap
  (params (OtherActor :type Actor%20Object%20Reference)))

(event EventTick
  (params (DeltaSeconds :type Float%20%28single-precision%29)))

(fn ConstructionScript)