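; BP_PickupObject is a collectible detail item that the player can pick up.
; Pickup calls DetailAdd on the ThirdPersonCharacter with the item's Index, then destroys the actor.
; In the Printer level it also clears the Blocked flag on the printer reference, which its creator supplies through Assign.
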(event Custom|Pickup
  (bind _asthird_person_character (Utilities|Casting|CastToThirdPersonCharacter (Game|Player|GetPlayerPawn 0)))
  (Default|DetailAdd _asthird_person_character (Variables|Default|Getindex))
  (bind _returnvalue (Game|GetCurrentLevelName true))
  (if (Utilities|Enum|Equal(Enum) _returnvalue "Printer")
    (Variables|/Game/Blueprint/BP_PrinterGoButton.BP_PrinterGoButton_C|Setblocked (Variables|Default|GetPrinter%20Ref) false))
  (Actor|DestroyActor))

(event Custom|Assign
  (params (Creator :type BP%20Printer%20Go%20Button%20Object%20Reference))
  (Variables|Default|SetPrinter%20ref Creator))

(event Collision|EventActorBeginOverlap
  (params (OtherActor :type Actor%20Object%20Reference)))

(event EventTick
  (params (DeltaSeconds :type Float%20%28single-precision%29)))

(fn ConstructionScript)