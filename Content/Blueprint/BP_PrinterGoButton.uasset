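; Printer go button that starts a print on its target and spawns the selected pickup object after a fixed delay.
; Pressing while blocked or already printing raises a mistake on the player character instead.
; A clamped index picks the mesh, temporarily offset by ten to a second set unless listed in NoSupportIndexes.
; Each spawned object is assigned this button and leaves it blocked.
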(event Custom|Spawn
  (bind _returnvalue (Game|Player|GetPlayerPawn 0))
  (if (Variables|Default|Getblocked)
    (bind _asthird_person_character (Utilities|Casting|CastToThirdPersonCharacter _returnvalue))
    (Default|RaiseMistake _asthird_person_character 2)
    (elif (Variables|Default|Getprinting)
      (bind _asthird_person_character_2 (Utilities|Casting|CastToThirdPersonCharacter _returnvalue))
      (Default|RaiseMistake _asthird_person_character_2 6)
      (else
        (Default|Print (Variables|Default|GetTarget))
        (Variables|Default|Setprinting true)
        (Utilities|FlowControl|Delay 12.0)
        (bind _returnvalue_2 (Game|SpawnActorfromClass "/Game/Blueprint/BP_PickupObject.BP_PickupObject_C" (Math|Transform|MakeTransform "-240.000000,600.000000,241.750000") "Undefined" 0 0))
        (Variables|Default|Setprinting false)
        (if (== (Utilities|Array|FindItem (Variables|Default|GetNo%20Support%20indexes) (Variables|Default|Getcurrent_index)) -1)
          (Variables|Default|Setcurrent_index (+ (Variables|Default|Getcurrent_index) 10)))
        (Default|Assign _returnvalue_2 self)
        (Components|StaticMesh|SetStaticMesh (Variables|/Game/Blueprint/BP_PickupObject.BP_PickupObject_C|GetStaticMesh _returnvalue_2) (Utilities|Array|Get(acopy) (Variables|/Game/Blueprint/BP_PickupObject.BP_PickupObject_C|Getmesh_list _returnvalue_2) (Variables|Default|Getcurrent_index)))
        (Variables|/Game/Blueprint/BP_PickupObject.BP_PickupObject_C|Setindex _returnvalue_2 (Variables|Default|Getcurrent_index))
        (Variables|Default|Setblocked true)
        (if (>= (Variables|Default|Getcurrent_index) 10)
          (Variables|Default|Setcurrent_index (- (Variables|Default|Getcurrent_index) 10)))))))

(event Custom|Press)

(event Custom|IndexChange
  (params (ispositive :type Boolean))
  (if ispositive
    (Variables|Default|Setcurrent_index (+ (Variables|Default|Getcurrent_index) 1))
    (if (== (Variables|Default|Getcurrent_index) 10)
      (Variables|Default|Setcurrent_index 9))
    (else
      (Variables|Default|Setcurrent_index (- (Variables|Default|Getcurrent_index) 1))
      (if (== (Variables|Default|Getcurrent_index) -1)
        (Variables|Default|Setcurrent_index 0)))))

(fn ConstructionScript)